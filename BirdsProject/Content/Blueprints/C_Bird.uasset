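; C_Bird is a bird pawn that can either be player-flown or fly in a flock.
; StartFlock raises movement speed, configures the FlockingBoid component with a leader, members and spacing, and opens a gate for flock updates, which StopFlock closes.
; When IsPlayer is set, Tick pushes the bird constantly forward and draws a debug forward trace.
; A provisional MoveAround event steers it by adding roll and pitch.
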(event Custom|MoveAround
  (params (NewParam :type Vector%202D%20Structure))
  ;[1 1 1] Provisoire
  (Class|Actor|AddActorWorldRotation (Math|Rotator|MakeRotator (.x NewParam) (.y NewParam) 0.0) false true))

(event Custom|StopFlock
  (bind _returnvalue (Transformation|GetActorLocation))
  (bind _returnvalue_2 (Transformation|GetActorForwardVector))
  ;[1 0.5341 0] Flocking
  (Utilities|FlowControl|Gate true ; enters at Close
    (:Exit
      (Class|FlockingBoid|Flock (Variables|Default|GetFlockingBoid) (stale EventTick DeltaSeconds))
      (if (Variables|Default|GetisPlayer)
        (Collision|LineTraceByChannel _returnvalue (+ _returnvalue (* _returnvalue_2 5e+03)) "TraceTypeQuery1" false 0 "ForOneFrame")
        (Class|PawnMovementComponent|AddInputVector (Variables|Default|GetFloatingPawnMovement) _returnvalue_2 true)))))

(event Custom|StartFlock
  (params (leader :type C%20Bird%20Object%20Reference) (flockMembers :type Array%20of%20Actor%20Object%20References))
  (bind _returnvalue (Transformation|GetActorLocation))
  (bind _returnvalue_2 (Transformation|GetActorForwardVector))
  (bind _floatingpawnmovement (Variables|Default|GetFloatingPawnMovement))
  ;[1 0.5341 0] Flocking
  (Variables|/Script/Engine.FloatingPawnMovement|SetMaxSpeed _floatingpawnmovement 1.2e+03)
  (Class|FlockingBoid|StartFlocking (Variables|Default|GetFlockingBoid) leader 15.0 15.0 15.0 flockMembers)
  (Utilities|FlowControl|Gate true ; enters at Open
    (:Exit
      (Class|FlockingBoid|Flock (Variables|Default|GetFlockingBoid) (stale EventTick DeltaSeconds))
      (if (Variables|Default|GetisPlayer)
        (Collision|LineTraceByChannel _returnvalue (+ _returnvalue (* _returnvalue_2 5e+03)) "TraceTypeQuery1" false 0 "ForOneFrame")
        (Class|PawnMovementComponent|AddInputVector _floatingpawnmovement _returnvalue_2 true)))))

(event EventBeginPlay
  (bind _asgm_in_game (Utilities|Casting|CastToGM_InGame (Game|GetGameMode)))
  (Variables|Default|SetAs%20GM%20In%20Game _asgm_in_game))

(event EventTick
  (params (DeltaSeconds :type Float%20%28single-precision%29))
  (bind _returnvalue (Transformation|GetActorLocation))
  (bind _returnvalue_2 (Transformation|GetActorForwardVector))
  ;[1 0.5341 0] Flocking
  (if (Variables|Default|GetisPlayer)
    (Collision|LineTraceByChannel _returnvalue (+ _returnvalue (* _returnvalue_2 5e+03)) "TraceTypeQuery1" false 0 "ForOneFrame")
    (Class|PawnMovementComponent|AddInputVector (Variables|Default|GetFloatingPawnMovement) _returnvalue_2 true)))

(fn ConstructionScript)