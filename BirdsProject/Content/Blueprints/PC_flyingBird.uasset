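; Player controller for a flying bird that steers the possessed bird's rotation from input, presumably the mouse.
; On BeginPlay it adds the Enhanced Input mapping context to the local player subsystem.
; The rotate action scales its 2D value by mouse sensitivity, mapping X to inverted roll and Y to pitch, with no yaw.
; It converts these angles to a quaternion and applies it as a local delta rotation to the bird.
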(event Input|EnhancedActionEvents|EnhancedInputActionAction_Rotate
  (params (ActionValue :type Vector%202D%20Structure) (ElapsedSeconds :type Float%20%28double-precision%29) (TriggeredSeconds :type Float%20%28double-precision%29) (InputAction :type Input%20Action%20Object%20Reference :default "/Game/Inputs/InputSystem/Action_Rotate.Action_Rotate"))
  (bind _mousesensibility (Variables|Default|GetMouseSensibility))
  (bind _returnvalue (* (Math|Vector2D|MakeVector2D (.x ActionValue) (.y ActionValue)) _mousesensibility))
  (bind _returnvalue_2 (Math|Rotator|MakeRotator (.x _returnvalue) (.y _returnvalue) 0.0))
  (bind _returnvalue_3 (Class|QuaternionInput|EulertoQuaternion (Math|Rotator|MakeRotator (.roll (* (Math|Rotator|MakeRotator (.roll _returnvalue_2) 0.0 0.0) -1.0)) (.pitch _returnvalue_2) (.yaw _returnvalue_2))))
  (Class|QuaternionInput|AddActorLocalRotationQuat (Variables|Default|GetQuaternionInput) (Variables|Default|GetpossededBird) _returnvalue_3))

(event EventBeginPlay
  ;[1 1 1] Add IMC
  (Input|AddMappingContext (PlayerController|LocalPlayerSubsystems|GetEnhancedInputLocalPlayerSubsystem) "/Game/Inputs/InputSystem/IMC.IMC" 0 "(bIgnoreAllPressedKeysUntilRelease=True,bForceImmediately=False,bNotifyUserSettings=False)"))

(fn ConstructionScript)